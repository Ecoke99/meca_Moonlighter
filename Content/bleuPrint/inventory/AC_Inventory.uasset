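; Inventory component that stores items in an array of slots and handles picking up new ones.
; TakeItem looks up a slot with the same ItemName and adds the incoming amount to it, with no stack limit check.
; Otherwise it writes the item into the first slot not flagged ItemValid, or prints "Inventaire Plein" when none is free.
; TakeItem has two item inputs: Item for lookup and new slots, Item1 for the amount added.
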(fn `AddItemIndex`
  (params (Item :type "/Game/bleuPrint/inventory/S_Item Structure") (Index :type Integer))
  (bind _output (`|GetArrayItem` (`self.Array`) Index))
  (bind _structout (setmembers `/Game/bleuPrint/inventory/S_Item` :`StructRef` _output :`ItemAmount` (+ (`.ItemAmount_9_71724AEC40AFE730B2E20DABFC8E306C` (break `/Game/bleuPrint/inventory/S_Item` Item)) (`.ItemAmount_9_71724AEC40AFE730B2E20DABFC8E306C` (break `/Game/bleuPrint/inventory/S_Item` _output)))))
  (`KismetArrayLibrary.Array_Set` (`self.Array`) Index _structout))

(fn `FindEmptySlodes`
  (returns (Succes :type Boolean) (Index :type Integer))
  (for (_array_element _array_index) (`self.Array`)
    (if (not (`.ItemValid_12_12413A644BAD8DE733816DBFCADA1FBB` (break `/Game/bleuPrint/inventory/S_Item` _array_element)))
      (return true _array_index))))

(fn `FindItem`
  (params (Item :type "/Game/bleuPrint/inventory/S_Item Structure"))
  (returns (Find :type Boolean) (Index :type Integer))
  (for (_array_element _array_index) (`self.Array`)
    (if (`KismetTextLibrary.EqualEqual_TextText` (`.ItemName_2_CD37925A4C1D54A6E76514ACB0956275` (break `/Game/bleuPrint/inventory/S_Item` _array_element)) (`.ItemName_2_CD37925A4C1D54A6E76514ACB0956275` (break `/Game/bleuPrint/inventory/S_Item` Item)))
      (return true _array_index))))

(fn `TakeItem`
  (params (Item :type "/Game/bleuPrint/inventory/S_Item Structure") (Item1 :type "/Game/bleuPrint/inventory/S_Item Structure"))
  (bind (_find _index) (`self.FindItem` Item))
  (if _find
    (`self.AddItemIndex` Item1 _index)
    (else
      (bind (_succes _index_2) (`self.FindEmptySlodes`))
      (if _succes
        (`KismetArrayLibrary.Array_Set` (`self.Array`) _index_2 (`local.Item`))
        (else
          (`KismetSystemLibrary.PrintText` "Inventaire Plein"))))))